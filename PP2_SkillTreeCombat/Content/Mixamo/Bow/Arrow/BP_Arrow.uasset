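; Bow arrow actor that flies when fired, damages what it overlaps and stops at the impact point.
; An In Bow / In Air / In Object state machine switches collision and creates or destroys the projectile movement component.
; Fire launches it forward at a speed scaled by bow charge.
; Overlaps in flight ignore the player, apply adjustable damage, offset the arrow back from impact and call attach.
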(event OnComponentBeginOverlap(Arrow)
  (params (OverlappedComponent :type Primitive%20Component%20Object%20Reference) (OtherActor :type Actor%20Object%20Reference) (OtherComp :type Primitive%20Component%20Object%20Reference) (OtherBodyIndex :type Integer) (bFromSweep :type Boolean) (SweepResult :type Hit%20Result%20Structure%20%28by%20ref%29))
  (CallFunction|HandleOverlap OtherActor SweepResult))

(event Custom|Fire
  (params (Charge :type Float%20%28single-precision%29))
  (Variables|Default|SetBowCharge Charge)
  (CallFunction|SetArrowState "NewEnumerator3"))

(event Custom|Increase%20Arrow%20Damage
  (params (add%20value :type Float%20%28single-precision%29))
  (Variables|Default|SetArrow%20Damage (+ (Variables|Default|GetArrow%20Damage) add%20value)))

(fn ConstructionScript)

(fn SetArrowState
  (params (State :type ENUM_ArrowState%20Enum :default "NewEnumerator0"))
  (if (Utilities|Enum|NotEqual(Enum) State (Variables|Default|GetArrowState))
    (CallFunction|OnStateEnd (Variables|Default|GetArrowState))
    (bind _output_get (Variables|Default|SetArrowState State))
    (CallFunction|OnStateBegin _output_get)))

(fn OnStateBegin
  (params (State :type ENUM_ArrowState%20Enum :default "NewEnumerator0"))
  (switch Utilities|FlowControl|Switch|SwitchonENUM_ArrowState State
    (:NewEnumerator1
      (Collision|SetCollisionProfileName (Variables|Default|GetArrow) "NoCollision" false :!class /Script/Engine.PrimitiveComponent))
    (:NewEnumerator2
      (Collision|SetCollisionProfileName (Variables|Default|GetArrow) "NoCollision" false :!class /Script/Engine.PrimitiveComponent))
    (:NewEnumerator3
      (Collision|SetCollisionProfileName (Variables|Default|GetArrow) "OverlapAllDynamic" false :!class /Script/Engine.PrimitiveComponent)
      (bind _returnvalue (AddComponent|AddProjectileMovementComponent))
      (bind _output_get (Variables|Default|SetProjectileComponate _returnvalue))
      (Variables|/Script/Engine.MovementComponent|SetVelocity _output_get (* (Transformation|GetActorForwardVector) (Math|Float|Lerp 1e+02 4e+03 (Variables|Default|GetBowCharge))))
      (Variables|/Script/Engine.ProjectileMovementComponent|SetbRotationFollowsVelocity _output_get true))))

(fn OnStateEnd
  (params (State :type ENUM_ArrowState%20Enum :default "NewEnumerator0"))
  (switch Utilities|FlowControl|Switch|SwitchonENUM_ArrowState State
    (:NewEnumerator3
      (Components|DestroyComponent (Variables|Default|GetProjectileComponate)))))

(fn HandleOverlap
  (params (Other%20Actor :type Actor%20Object%20Reference) (Hit%20Result :type Hit%20Result%20Structure))
  (switch Utilities|FlowControl|Switch|SwitchonENUM_ArrowState (Variables|Default|GetArrowState)
    (:NewEnumerator3
      (if (!= Other%20Actor (Game|GetPlayerCharacter 0))
        (Game|Damage|ApplyDamage Other%20Actor (Variables|Default|GetArrow%20Damage) 0 0)
        (CallFunction|SetArrowState "NewEnumerator1")
        (Transformation|SetActorLocation (- (.ImpactPoint (Collision|BreakHitResult Hit%20Result)) (* (Transformation|GetActorForwardVector) 5e+01)) false true)
        (Transformation|AttachActorToActor 0 "None" "KeepWorld" "KeepWorld" "KeepWorld" true)))))