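; Player bow actor that nocks, charges and fires arrows, with upgrade hooks for arrow scale, draw speed and damage.
; Reload events spawn single, double, quad or nine-shot arrow actors at the current scale and attach them to the nock socket.
; A Charge timeline drives ChargeAmount, and shortening it speeds up the draw.
; Fire detaches the arrow, adds one skill-tree damage bonus, launches it with ChargeAmount and resets the charge.
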(event Custom|BeginCharge
  (Variables|Default|GetArrowInBow
    (:then
      (bind _chargeamount (Timeline|Charge Play)
        (:Update
          (Variables|Default|SetCharge%20Amount _chargeamount))))
    (:else)))

(event Custom|EndCharge
  (Variables|Default|GetArrowInBow
    (:then
      (bind _chargeamount (Timeline|Charge Reverse)
        (:Update
          (Variables|Default|SetCharge%20Amount _chargeamount))))
    (:else)))

(event Custom|StopCharge
  (Utilities|FlowControl|Sequence
    (:then_0
      (bind _chargeamount (Timeline|Charge Stop)
        (:Update
          (Variables|Default|SetCharge%20Amount _chargeamount))))
    (:then_1
      (Timeline|Charge SetNewTime))))

(event Custom|Fire
  (bind _arrowinbow (Variables|Default|GetArrowInBow)
    (:then
      (Transformation|DetachFromActor _arrowinbow "KeepWorld" "KeepWorld" "KeepWorld")
      (bind _asthird_person_character (Utilities|Casting|CastToThirdPersonCharacter (Game|GetPlayerCharacter 0)))
      (if (Variables|/Game/UI/Blueprints/SkillButton.SkillButton_C|Getaquired (Variables|/Game/UI/Blueprints/SkilltreeUI.SkilltreeUI_C|GetDamageIIButton (Variables|/Game/ThirdPersonBP/Blueprints/ThirdPersonCharacter.ThirdPersonCharacter_C|GetSkilltreeUI _asthird_person_character)))
        (Default|IncreaseArrowDamage (Variables|Default|GetArrowInBow) 1e+01)
        (elif (Variables|/Game/UI/Blueprints/SkillButton.SkillButton_C|Getaquired (Variables|/Game/UI/Blueprints/SkilltreeUI.SkilltreeUI_C|GetDamageIButton (Variables|/Game/ThirdPersonBP/Blueprints/ThirdPersonCharacter.ThirdPersonCharacter_C|GetSkilltreeUI _asthird_person_character)))
          (Default|IncreaseArrowDamage (Variables|Default|GetArrowInBow) 5.0)
          (elif (Variables|/Game/UI/Blueprints/SkillButton.SkillButton_C|Getaquired (Variables|/Game/UI/Blueprints/SkilltreeUI.SkilltreeUI_C|GetIncreaseDamageandSizeFinalButton (Variables|/Game/ThirdPersonBP/Blueprints/ThirdPersonCharacter.ThirdPersonCharacter_C|GetSkilltreeUI _asthird_person_character)))
            (Default|IncreaseArrowDamage (Variables|Default|GetArrowInBow) 15.0))))
      (Default|Fire (Variables|Default|GetArrowInBow) (Variables|Default|GetCharge%20Amount))
      (Variables|Default|SetArrowInBow 0)
      (CallFunction|StopCharge))
    (:else)))

(event Custom|Reload
  (bind _scale (Variables|Default|GetScale))
  (bind _returnvalue (Game|SpawnActorfromClass "/Game/Mixamo/Bow/Arrow/BP_Arrow.BP_Arrow_C" (Math|Transform|MakeTransform "0, 0, 0" "0, 0, 0" (Math|Vector|MakeVector 1.0 _scale _scale)) "Undefined" 0 "NewEnumerator2" 0))
  (bind _output_get (Variables|Default|SetArrowInBow _returnvalue))
  (Transformation|AttachComponentToComponent _output_get (Variables|Default|GetBow) "ArrowNockPoint" "SnapToTarget" "SnapToTarget" "KeepWorld" true))

(event Custom|Quad%20Reload
  (bind _scale (Variables|Default|GetScale))
  (bind _returnvalue (Game|SpawnActorfromClass "/Game/Mixamo/Bow/Arrow/QuadArrow.QuadArrow_C" (Math|Transform|MakeTransform "0, 0, 0" "0, 0, 0" (Math|Vector|MakeVector 1.0 _scale _scale)) "Undefined" 0 "NewEnumerator2" 0))
  (bind _output_get (Variables|Default|SetArrowInBow _returnvalue))
  (Transformation|AttachComponentToComponent _output_get (Variables|Default|GetBow) "ArrowNockPoint" "SnapToTarget" "SnapToTarget" "KeepWorld" true))

(event Custom|9%20Shot
  (bind _scale (Variables|Default|GetScale))
  (bind _returnvalue (Game|SpawnActorfromClass "/Game/Mixamo/Bow/Arrow/9_Arrow.9_Arrow_C" (Math|Transform|MakeTransform "0, 0, 0" "0, 0, 0" (Math|Vector|MakeVector 1.0 _scale _scale)) "Undefined" 0 "NewEnumerator2" 0))
  (bind _output_get (Variables|Default|SetArrowInBow _returnvalue))
  (Transformation|AttachComponentToComponent _output_get (Variables|Default|GetBow) "ArrowNockPoint" "SnapToTarget" "SnapToTarget" "KeepWorld" true))

(event Custom|Double%20Shot
  (bind _scale (Variables|Default|GetScale))
  (bind _returnvalue (Game|SpawnActorfromClass "/Game/Mixamo/Bow/Arrow/Double_Arrow.Double_Arrow_C" (Math|Transform|MakeTransform "0, 0, 0" "0, 0, 0" (Math|Vector|MakeVector 1.0 _scale _scale)) "Undefined" 0 "NewEnumerator2" 0))
  (bind _output_get (Variables|Default|SetArrowInBow _returnvalue))
  (Transformation|AttachComponentToComponent _output_get (Variables|Default|GetBow) "ArrowNockPoint" "SnapToTarget" "SnapToTarget" "KeepWorld" true))

(event Custom|Decrese%20Draw%20Speed
  (bind _charge (Variables|Default|GetCharge))
  (Components|Timeline|SetTimelineLength _charge (- (Components|Timeline|GetTimelineLength _charge) 0.5)))

(event Custom|Increase%20Scale
  (params (Additon%20Scale :type Float%20%28single-precision%29))
  (Variables|Default|SetScale (+ (Variables|Default|GetScale) Additon%20Scale)))

(fn ConstructionScript)